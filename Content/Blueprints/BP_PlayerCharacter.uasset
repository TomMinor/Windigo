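; Player character Blueprint that switches first-person cameras around jumps and hosts a debug world-trace test.
; Jumping activates FirstPersonCameraBP, intended to snap the view to the head, and landing restores FirstPersonCameraComponent.
; When EnableTraceTest is set, Tick box-traces a unit forward from FirstPersonCameraComponent, sized by IkWorldCheckBBox, and draws the first hit actor's name at the impact.
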(event EventOnJumped
  ;[1 1 1] Snap camera to head when the player jumps
  (Components|Activation|Deactivate (Variables|Default|GetFirstPersonCameraComponent))
  (Components|Activation|SetActive (Variables|Default|GetFirstPersonCamera_BP) true false))

(event EventOnLanded
  (params (Hit :type Hit%20Result%20Structure%20%28by%20ref%29))
  ;[1 1 1] Snap camera to head when the player jumps
  (Components|Activation|Deactivate (Variables|Default|GetFirstPersonCamera_BP))
  (Components|Activation|SetActive (Variables|Default|GetFirstPersonCameraComponent) true false))

(event EventTick
  (params (DeltaSeconds :type Float%20%28single-precision%29))
  (bind _firstpersoncameracomponent (Variables|Default|GetFirstPersonCameraComponent))
  (bind _returnvalue (Transformation|GetWorldLocation _firstpersoncameracomponent))
  (bind _returnvalue_2 (Transformation|GetWorldRotation _firstpersoncameracomponent))
  (bind _returnvalue_3 (Math|Vector|GetForwardVector _returnvalue_2))
  (if (Variables|Default|GetEnableTraceTest)
    (bind _outhits (Class|KismetSystemLibrary|BoxTraceMulti _returnvalue (+ _returnvalue _returnvalue_3) (Variables|Default|GetikWorldCheckBBox) (Math|Conversions|RotationFromXVector (.Y (Math|Rotator|BreakRotIntoAxes (Math|Conversions|RotationFromXVector _returnvalue_3)))) "TraceTypeQuery1" false 0 "None" true))
    ;[1 1 1] Retrieve the first object we hit
    (Rendering|Debug|DrawDebugString (.Location (Collision|BreakHitResult (Utilities|Array|Get(acopy) _outhits))) (Utilities|GetDisplayName (.HitActor (Collision|BreakHitResult (Utilities|Array|Get(acopy) _outhits)))) 0 "(R=1.000000,G=0.000000,B=0.000000,A=1.000000)" 1.0)))

(fn ConstructionScript)